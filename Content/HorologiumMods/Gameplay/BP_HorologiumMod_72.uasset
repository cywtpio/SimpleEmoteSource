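; Horologium mod Blueprint that lets the player trigger dance emotes (Griddy, Floss, L, Electro) on their character with hotkeys.
; Each Tick it polls player 0's H, J, K and L keys and plays the matching animation once on the character mesh.
; A fixed four-second delay then restores Animation Blueprint mode, and P restores it immediately.
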(event `self.ReceiveTick`
  (params (DeltaSeconds :type "Float (single-precision)"))
  (bind _mesh (`Character.Mesh` (`GameplayStatics.GetPlayerCharacter` 0)))
  (bind _mesh_2 (`Character.Mesh` (`GameplayStatics.GetPlayerCharacter` 0)))
  (bind _mesh_3 (`Character.Mesh` (`GameplayStatics.GetPlayerCharacter` 0)))
  (bind _mesh_4 (`Character.Mesh` (`GameplayStatics.GetPlayerCharacter` 0)))
  (`|ExecutionSequence`
    (:`then_0`
      (if (`PlayerController.WasInputKeyJustPressed` (`GameplayStatics.GetPlayerController` 0) "H")
        (`SkeletalMeshComponent.PlayAnimation` _mesh_2 "/Game/Characters/Campers/Common/EmoteV2/Griddy/GriddyAnim.GriddyAnim" false)
        (`KismetSystemLibrary.Delay` 4.0)
        (`SkeletalMeshComponent.SetAnimationMode` _mesh_2 "AnimationBlueprint")))
    (:`then_1`
      (if (`PlayerController.WasInputKeyJustPressed` (`GameplayStatics.GetPlayerController` 0) "J")
        (`SkeletalMeshComponent.PlayAnimation` _mesh_3 "/Game/Characters/Campers/Common/EmoteV2/Floss/FlossAnim.FlossAnim" false)
        (`KismetSystemLibrary.Delay` 4.0)
        (`SkeletalMeshComponent.SetAnimationMode` _mesh_3 "AnimationBlueprint")))
    (:`then_2`
      (if (`PlayerController.WasInputKeyJustPressed` (`GameplayStatics.GetPlayerController` 0) "K")
        (`SkeletalMeshComponent.PlayAnimation` _mesh "/Game/Characters/Campers/Common/EmoteV2/L/LAnim.LAnim" false)
        (`KismetSystemLibrary.Delay` 4.0)
        (`SkeletalMeshComponent.SetAnimationMode` _mesh "AnimationBlueprint")))
    (:`then_3`
      (if (`PlayerController.WasInputKeyJustPressed` (`GameplayStatics.GetPlayerController` 0) "P")
        (`SkeletalMeshComponent.SetAnimationMode` (`Character.Mesh` (`GameplayStatics.GetPlayerCharacter` 0)) "AnimationBlueprint")))
    (:`then_4`
      (if (`PlayerController.WasInputKeyJustPressed` (`GameplayStatics.GetPlayerController` 0) "L")
        (`SkeletalMeshComponent.PlayAnimation` _mesh_4 "/Game/Characters/Campers/Common/EmoteV2/Electro/ElectroAnim.ElectroAnim" false)
        (`KismetSystemLibrary.Delay` 4.0)
        (`SkeletalMeshComponent.SetAnimationMode` _mesh_4 "AnimationBlueprint")))))

(fn `UserConstructionScript`)